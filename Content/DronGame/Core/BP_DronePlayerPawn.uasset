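; BP_DronePlayerPawn is a player drone pawn that adds on-screen debug readouts and a camera view toggle.
; Tick prints throttle from DroneMovementComponent, speed from BoxComponent velocity and health from HealthComponent, using keyed messages.
; Despite its name, IA_ReloadLevel drives a FlipFlop that switches SpringArmComponent length and height between an extended chase view and a zero-length view.
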(event Input|EnhancedActionEvents|EnhancedInputActionIA_ReloadLevel
  (params (ActionValue :type Boolean) (ElapsedSeconds :type Float%20%28double-precision%29) (TriggeredSeconds :type Float%20%28double-precision%29) (InputAction :type Input%20Action%20Object%20Reference :default "/Game/DronGame/Input/InputActions/IA_ReloadLevel.IA_ReloadLevel"))
  (bind _springarmcomponent (Variables|Default|GetSpringArmComponent))
  (bind _springarmcomponent_2 (Variables|Default|GetSpringArmComponent))
  (:Triggered
    (Utilities|FlowControl|FlipFlop
      (:A
        (Variables|/Script/Engine.SpringArmComponent|SetTargetArmLength _springarmcomponent_2 3e+02)
        (Transformation|SetRelativeLocation _springarmcomponent_2 (Math|Vector|MakeVector 0.0 0.0 4e+01) false false))
      (:B
        (Variables|/Script/Engine.SpringArmComponent|SetTargetArmLength _springarmcomponent 0.0)
        (Transformation|SetRelativeLocation _springarmcomponent (Math|Vector|MakeVector 0.0 0.0 1e+01) false false)))))

(event EventBeginPlay)

(event Collision|EventActorBeginOverlap
  (params (OtherActor :type Actor%20Object%20Reference)))

(event EventTick
  (params (DeltaSeconds :type Float%20%28single-precision%29))
  (Development|PrintString (Utilities|String|Append "Throttle debug: " (Utilities|String|ToString(Float) (Variables|/Script/DroneGame.DroneMovementComponent|GetCurrentThrottle (Variables|Default|GetDroneMovementComponent)))) true false "(R=1.000000,G=0.795953,B=0.000000,A=1.000000)" -1.0 "1")
  (Development|PrintString (Utilities|String|Append "Throttle: " (Utilities|String|ToString(Float) (Class|DroneMovementComponent|GetThrottlePercent (Variables|Default|GetDroneMovementComponent)))) true false "(R=0.000000,G=1.000000,B=0.323219,A=1.000000)" -1.0 "2")
  (Development|PrintString (Utilities|String|Append "Speed: " (Utilities|String|ToString(Float) (Math|Vector|VectorLength (Transformation|GetComponentVelocity (Variables|Default|GetBoxComponent))))) true false "(R=1.000000,G=0.404302,B=0.000000,A=1.000000)" -1.0 "3")
  (Development|PrintString (Utilities|String|Append "Health: " (Utilities|String|ToString(Float) (Variables|/Script/DroneGame.HealthComponent|GetCurrentHealth (Variables|Default|GetHealthComponent)))) true true "(R=0.000000,G=1.000000,B=0.149880,A=1.000000)" -1.0 "4"))

(fn ConstructionScript)