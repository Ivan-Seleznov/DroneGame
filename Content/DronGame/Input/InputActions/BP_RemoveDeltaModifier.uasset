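; Enhanced Input modifier that removes the frame delta from an input action value, likely turning per-frame deltas into rates.
; ModifyRaw divides X and Y by DeltaTime and multiplies them by Scale, keeping the original value type.
; Z is computed inversely, as DeltaTime divided by Z times Scale, unlike the other two axes.
; No guard against a zero divisor is present.
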(fn ModifyRaw
  (params (PlayerInput :type Enhanced%20Player%20Input%20Object%20Reference) (CurrentValue :type Input%20Action%20Value%20Structure) (DeltaTime :type Float%20%28single-precision%29))
  (bind (_x _y _z _type) (Class|EnhancedInputLibrary|BreakInputActionValue CurrentValue))
  (bind _scale (Variables|Default|GetScale))
  (return (Class|EnhancedInputLibrary|MakeInputActionValueOfType (* (/ _x DeltaTime) _scale) (* (/ _y DeltaTime) _scale) (* (/ DeltaTime _z) _scale) _type)))